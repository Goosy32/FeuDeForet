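; BP_Tuto_Overlap is a tutorial trigger actor that advances the tutorial once two different players have passed through it.
; On begin overlap, it records each BP_ThirdPersonCharacter once in PlayersOverlapped and never removes it, so the players need not overlap simultaneously.
; When the second is added, it calls CallDISNextTask on BP_ThirdPersonGameMode and prints a debug message.
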(event `self.ReceiveActorBeginOverlap`
  (params (OtherActor :type "Actor Object Reference"))
  ; Permet de vérifier quand les deux joueurs sont passés dessus pour acctiver la prochaine phase du tuto
  (bind _asbp_third_person_character (cast `/Game/Game_Content/BP_ThirdPersonCharacter` OtherActor))
  (if (not (`KismetArrayLibrary.Array_Contains` (`self.PlayersOverlapped`) _asbp_third_person_character))
    (bind _output_get (set `self.PlayersOverlapped` (`self.PlayersOverlapped`)))
    (`KismetArrayLibrary.Array_Add` _output_get _asbp_third_person_character)
    (if (== (`KismetArrayLibrary.Array_Length` (`self.PlayersOverlapped`)) 2)
      (bind _asbp_third_person_game_mode (cast `/Game/Game_Content/BP_ThirdPersonGameMode` (`GameplayStatics.GetGameMode`)))
      (`/Game/Game_Content/BP_ThirdPersonGameMode.DIS_NextTask` _asbp_third_person_game_mode)
      (`KismetSystemLibrary.PrintString` "Task"))))

(fn `UserConstructionScript`)