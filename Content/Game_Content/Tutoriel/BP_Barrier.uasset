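; BP_Barrier is a tutorial barrier actor that removes itself once the task number set in TaskVal is reached.
; With a TaskVal of zero, it destroys itself shortly after BeginPlay.
; Otherwise it binds to the DISNextTask dispatcher on BP_ThirdPersonGameMode and increments its own task counter on each call.
; After a short delay, it destroys itself if that counter matches TaskVal.
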(event `self.ReceiveBeginPlay`
  (if (== (`self.TaskVal`) 0)
    (`KismetSystemLibrary.Delay` 7.0)
    (`self.K2_DestroyActor`)
    (else
      (bind _asbp_third_person_game_mode (cast `/Game/Game_Content/BP_ThirdPersonGameMode` (`GameplayStatics.GetGameMode`)))
      (add `/Game/Game_Content/BP_ThirdPersonGameMode.DIS_NextTask` _asbp_third_person_game_mode (delegate `DeleteBarrier`)))))

(event `DeleteBarrier`
  (set `self.CurrentTask` (+ (`self.CurrentTask`) 1))
  (`KismetSystemLibrary.Delay` 6.0)
  (if (== (`self.CurrentTask`) (`self.TaskVal`))
    (`self.K2_DestroyActor`)))

(fn `UserConstructionScript`)