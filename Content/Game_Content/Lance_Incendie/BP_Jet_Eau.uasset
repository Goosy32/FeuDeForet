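; Water jet projectile of the fire hose that fights fires and affects characters it hits.
; Tick accumulates lifetime and destroys the actor once LifeTimeMax is exceeded.
; Its Box overlap shrinks any BP_Fire through a negative FireGrow.
; A BP_ThirdPersonCharacter hit is extinguished if burning, otherwise launched away from the jet along the normalized offset, and the jet is destroyed either way.
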(event `self.ReceiveTick`
  (params (DeltaSeconds :type "Float (single-precision)"))
  (set `self.LifeTime` (+ DeltaSeconds (`self.LifeTime`)))
  (if (> (`self.LifeTime`) (`self.LifeTimeMax`))
    (`self.K2_DestroyActor`)))

(event `self.ReceiveBeginPlay`
  (set `self.LifeTime` 0.0))

(event `self.Box.OnComponentBeginOverlap`
  (params (OverlappedComponent :type "PrimitiveComponent Object Reference") (OtherActor :type "Actor Object Reference") (OtherComp :type "PrimitiveComponent Object Reference") (OtherBodyIndex :type Integer) (bFromSweep :type Boolean) (SweepResult :type "HitResult Structure (by ref)"))
  (`|ExecutionSequence`
    (:`then_0`
      (bind _asbp_fire (cast `/Game/Game_Content/Feu/BP_Fire` OtherActor))
      (`/Game/Game_Content/Feu/BP_Fire.FireGrow` _asbp_fire -0.05))
    (:`then_1`
      (bind _asbp_third_person_character (cast `/Game/Game_Content/BP_ThirdPersonCharacter` OtherActor))
      (if (`/Game/Game_Content/BP_ThirdPersonCharacter.IsOnFire` _asbp_third_person_character)
        (`/Game/Game_Content/BP_ThirdPersonCharacter.ExtinguishFire` _asbp_third_person_character)
        (`self.K2_DestroyActor`)
        (else
          (bind _returnvalue (* (`KismetMathLibrary.Normal` (`KismetMathLibrary.MakeVector` (.x (- (`self.K2_GetActorLocation` _asbp_third_person_character) (`self.K2_GetActorLocation`))) (.y (- (`self.K2_GetActorLocation` _asbp_third_person_character) (`self.K2_GetActorLocation`))) (.z (- (`self.K2_GetActorLocation` _asbp_third_person_character) (`self.K2_GetActorLocation`))))) 100.0))
          (`Character.LaunchCharacter` _asbp_third_person_character _returnvalue false false)
          (`KismetSystemLibrary.PrintString` (`KismetStringLibrary.Conv_VectorToString` _returnvalue))
          (`self.K2_DestroyActor`))))))

(fn `UserConstructionScript`)