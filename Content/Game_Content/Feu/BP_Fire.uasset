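; BP_Fire is a fire actor that tracks its own growth as a value from zero to one.
; BeginPlay sets a timer, with no looping specified, to call FirePropagation after a hundredth of TimeToMaxGrowth.
; FirePropagation calls FireGrow below full growth, which adds one percent and clamps the result.
; Despite the event's name, nothing spreads, and the node scaling the Cube by growth is disconnected.
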(event `self.ReceiveBeginPlay`
  (`KismetSystemLibrary.K2_SetTimerDelegate` (delegate `FirePropagation`) (/ (`self.TimeToMaxGrowth`) 100.0)))

(event `FirePropagation`
  (if (< (`self.FireGrowth`) 1.0)
    (`self.FireGrow`)))

(fn `FireGrow`
  (set `self.FireGrowth` (`KismetMathLibrary.FClamp` (+ (`self.FireGrowth`) 0.01))))

(fn `UserConstructionScript`)